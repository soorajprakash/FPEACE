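; Gameplay ability that makes an enemy perform an attack and ends if the enemy gains the TakingDamage tag.
; On activation it starts a tag listener, then commits the ability and plays a random attack montage on the main body mesh.
; The montage start triggers a crossfaded zombie attack vocal, and blend-out or completion ends the ability.
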(event Ability|EventActivateAbility
  (Ability|Tasks|WaitGameplayTagAdd "(TagName=\"Character.Enemy.TakingDamage\")" 0
    (:then
      (bind _returnvalue (Ability|CommitAbility))
      (if _returnvalue
        (Animation|Montage|PlayMontage (Variables|Default|GetEnemyMainBodyMesh) (.OutItem (Utilities|Array|Random (Variables|Default|GetAttackMontages)))
          (:then
            (Class|FPCCharacter|PlayVocalSound (Variables|Default|GetFPCEnemyCharacter) "/Game/FPEACE/Audio/Gameplay/Enemies/MetaSounds/Zombie_Attacks.Zombie_Attacks" 1.0))
          (:OnCompleted
            (Ability|EndAbility :!label _label))
          (:OnBlendOut
            (goto _label)))))
    (:Added
      (Ability|EndAbility))))
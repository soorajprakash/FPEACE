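; Base enemy character Blueprint for pooled zombie enemies, linking GAS, montages, vocal audio and StateTree AI.
; On spawn from the pool it chains crawl-out and stand-up montages, then starts StateTree logic, which death stops while fading vocals.
; Hits play a reaction montage and apply a hit-taken effect intended to match its length.
; It also hands its ability system to the health bar widget and growls on entering chase.
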(event Custom|EnteredChasingState
  (Class|FPCCharacter|PlayVocalSound "/Game/FPEACE/Audio/Gameplay/Enemies/MetaSounds/Zombie_Growls.Zombie_Growls" 1.0))

(event EventBeginPlay
  (Utilities|FlowControl|Sequence
    (:then_0
      ;[0 0 0 1 14] Initialize the viewmodel for the healthbar
      (bind _aswbp_enemy_health_bar (Utilities|Casting|CastToWBP_EnemyHealthBar (UserInterface|GetUserWidgetObject (Variables|Default|GetHealthBarWidgetComp))))
      (Variables|/Game/FPEACE/Art/UI/Widgets/3D/WBP_EnemyHealthBar.WBP_EnemyHealthBar_C|SetOwningASC _aswbp_enemy_health_bar (Variables|Default|GetFPCAbilitySystemComponent)))))

(event EventOnHitDamageTaken
  (params (HitReactionMontage :type Anim%20Montage%20Object%20Reference))
  (bind _fpcabilitysystemcomponent (Variables|Default|GetFPCAbilitySystemComponent))
  (bind _returnvalue (GameplayEffects|MakeOutgoingSpec :self _fpcabilitysystemcomponent :GameplayEffectClass "/Game/FPEACE/Art/Enemies/GAS/GE_EnemyHitTaken.GE_EnemyHitTaken_C"))
  (Ability|GameplayEffect|SetDuration _returnvalue (Animation|GetPlayLength HitReactionMontage))
  (GameplayEffects|ApplyGameplayEffectSpecToSelf _fpcabilitysystemcomponent _returnvalue)
  (Animation|Montage|PlayMontage (Variables|Default|GetMainBodyMeshComp) HitReactionMontage))

(event EventOnDeath
  (|CallParentFunction)
  (bind _asbp_enemy_aicontroller (Utilities|Casting|CastToBP_EnemyAIController (Pawn|GetController)))
  (AI|Logic|StopLogic (Variables|/Script/FPEACE.FPCEnemyAIController|GetStateTreeAIComp _asbp_enemy_aicontroller) "Enemy Character Died")
  (Audio|Components|Audio|FadeOut (Variables|Default|GetVocalAudioComponent) 1.0 0.0 "Linear" :!class /Script/Engine.AudioComponent))

(event EventOnPulledfromPool
  (bind _mainbodymeshcomp (Variables|Default|GetMainBodyMeshComp))
  (|CallParentFunction)
  ;[0 0 0 1 14] Play Spawn Montage
  (Animation|Montage|PlayMontage _mainbodymeshcomp "/Game/FPEACE/Art/Enemies/Zombie/Animations/Sequences/Zombie_Crawl/AM_Zombie_Crawl_OutOfGround_To_CrawlIdle.AM_Zombie_Crawl_OutOfGround_To_CrawlIdle"
    (:OnBlendOut
      (Animation|Montage|PlayMontage _mainbodymeshcomp "/Game/FPEACE/Art/Enemies/Zombie/Animations/Sequences/Zombie_Crawl/AM_Zombie_Crawl_CrawlIdle_To_Stand.AM_Zombie_Crawl_CrawlIdle_To_Stand"
        (:OnCompleted
          _)
        (:OnBlendOut
          _)
        (:OnInterrupted
          _)))
    (:OnInterrupted
      _))
  (bind _asbp_enemy_aicontroller (Utilities|Casting|CastToBP_EnemyAIController (Pawn|GetController)))
  (AI|Logic|StartLogic (Variables|/Script/FPEACE.FPCEnemyAIController|GetStateTreeAIComp _asbp_enemy_aicontroller)))

(fn ConstructionScript)
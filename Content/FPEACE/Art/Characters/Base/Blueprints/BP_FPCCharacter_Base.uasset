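; Base character Blueprint that handles which weapon the character has equipped.
; On BeginPlay it passes the default weapon class from its character data to the weapon manager component to equip.
; Hard-wired 1 and 2 key events call the same component to switch between the unarmed and pistol weapon classes.
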(event EventBeginPlay
  (Class|FPCCharacterWeaponManagerComponent|EquipWeapon (Variables|Default|GetFPCCharacterWeaponManagerComp) (Variables|/Script/FPEACE.FPCCharacterData|GetDefaultWeaponBP (Variables|Default|GetFPCCharacterData))))

(event Input|KeyboardEvents|1
  (params (Key :type Key%20Structure :default "None"))
  (:Pressed
    (Class|FPCCharacterWeaponManagerComponent|EquipWeapon (Variables|Default|GetFPCCharacterWeaponManagerComp) (Variables|Default|GetUnarmedWeaponClass))))

(event Input|KeyboardEvents|2
  (params (Key :type Key%20Structure :default "None"))
  (:Pressed
    (Class|FPCCharacterWeaponManagerComponent|EquipWeapon (Variables|Default|GetFPCCharacterWeaponManagerComp) (Variables|Default|GetPistolWeaponClass))))

(fn ConstructionScript)
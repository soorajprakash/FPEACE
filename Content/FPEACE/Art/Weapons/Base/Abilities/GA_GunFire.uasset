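; GA_GunFire is a gameplay ability that fires the referenced gun and rate-limits shots.
; On a successful commit it applies GE_FireCooldown to the owner, passing a SetByCaller cooldown magnitude equal to the reciprocal of a float attribute.
; It then calls Fire on GunRef and ends, while a failed commit has no handling and never calls EndAbility.
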(event Ability|EventActivateAbility
  (bind _returnvalue (Ability|CommitAbility))
  (if _returnvalue
    (bind _returnvalue_2 (Ability|GameplayEffect|AssignTagSetbyCallerMagnitude (Ability|MakeOutgoingGameplayEffectSpec "/Game/FPEACE/Art/Weapons/Base/GameplayEffects/GE_FireCooldown.GE_FireCooldown_C") "(TagName=\"DataTags.Weapon.Gun.Cooldown\")" (Math|Float|SafeDivide 1.0 (.ReturnValue (Ability|Attribute|GetFloatAttributefromAbilitySystemComponent (Ability|GetAbilitySystemComponentfromActorInfo) "(AttributeName=\"FireRate\",Attribute=/Script/FPEACE.FPCGunAttributeSet:FireRate,AttributeOwner=\"/Script/CoreUObject.Class'/Script/FPEACE.FPCGunAttributeSet'\")")))))
    (GameplayEffects|ApplyGameplayEffectSpecToSelf (Ability|GetAbilitySystemComponentfromActorInfo) _returnvalue_2)
    (Class|FPCGun|Fire (Variables|Default|GetGunRef))
    (Ability|EndAbility)))
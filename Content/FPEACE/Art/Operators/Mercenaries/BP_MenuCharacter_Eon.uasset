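; Menu display Blueprint for the mercenary operator Eon that gives the character a fixed facial expression.
; SetupFaceMorphs sets brow, eyelid and smile morph targets on OperatorMesh to form a slightly squinting, lopsided smile.
; It runs from the Construction Script, after the parent's, and again on BeginPlay, so the expression applies both at construction and at runtime.
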(event EventBeginPlay
  (CallFunction|SetupFaceMorphs))

(event Collision|EventActorBeginOverlap
  (params (OtherActor :type Actor%20Object%20Reference)))

(event EventTick
  (params (DeltaSeconds :type Float%20%28single-precision%29)))

(fn ConstructionScript
  (|CallParentFunction)
  (CallFunction|SetupFaceMorphs))

(fn SetupFaceMorphs
  (bind _operatormesh (Variables|Default|GetOperatorMesh))
  (Components|SkeletalMesh|SetMorphTarget _operatormesh "BrowOut_Up" 0.5 true)
  (Components|SkeletalMesh|SetMorphTarget _operatormesh "BrowCenter_Dn" 0.5 true)
  (Components|SkeletalMesh|SetMorphTarget _operatormesh "eyeBlinkLeft" 0.2 true)
  (Components|SkeletalMesh|SetMorphTarget _operatormesh "eyeBlinkRight" 0.2 true)
  (Components|SkeletalMesh|SetMorphTarget _operatormesh "mouthSmileLeft" 0.2 true)
  (Components|SkeletalMesh|SetMorphTarget _operatormesh "mouthSmileRight" 0.6 true))
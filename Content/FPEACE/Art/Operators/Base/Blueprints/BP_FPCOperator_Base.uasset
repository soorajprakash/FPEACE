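; Base operator character Blueprint that handles hit reactions and death presentation for playable operators.
; Taking damage plays a grunt and a hit montage on the main body mesh, throttled by a short delay gate.
; Death tweens global time dilation and post-process saturation down together for a slow-motion fade, then tells the gameplay player controller the game is over.
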(event EventOnHitDamageTaken
  (params (HitReactionMontage :type Anim%20Montage%20Object%20Reference))
  (if (Variables|Default|GetCanPlayDamageVocal)
    (Class|FPCCharacter|PlayVocalSound (Variables|Default|GetDamageTakenGrunt) 1.0)
    (Animation|Montage|PlayMontage (Variables|Default|GetMainBodyMeshComp) HitReactionMontage
      (:then
        (Variables|Default|SetCanPlayDamageVocal false)
        (Utilities|FlowControl|Delay 1.5)
        (Variables|Default|SetCanPlayDamageVocal true)))))

(event EventOnDeath
  (|CallParentFunction)
  (bind _value (|TweenFloat 1.0 0.025 2.0 "InOutQuad" 0.0 0.0 0.0 0 0.0 false 0.0 false false)
    (:ApplyEasing
      (Utilities|Time|SetGlobalTimeDilation _value)
      (Default|CallSetPostProcessSaturation _value))
    (:OnComplete
      (bind _asbp_gameplay_player_controller (Utilities|Casting|CastToBP_GameplayPlayerController (Game|GetInstigatorController)))
      (Default|OnGameOver _asbp_gameplay_player_controller))))

(fn ConstructionScript)
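; AI controller for enemy characters that chases the player operator or wanders the navmesh on request from calling tasks.
; It caches the possessed enemy and the player's pawn, then Tick updates a within-attack-distance flag from the distance between them.
; ChasePlayer and Wander use AIMoveTo toward the player or a random nearby navigable point.
; Both notify the calling task of completion whether the move succeeds or fails.
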(event Custom|Chase%20Player
  (params (CallingTask :type STT%20Chase%20Object%20Reference))
  (bind _playeroperatorref (Variables|Default|GetPlayerOperatorRef))
  (Utilities|IsValid _playeroperatorref
    (:Is%20Valid
      (AI|AIMoveTo (Variables|Default|GetControlledEnemyCharacter) (Transformation|GetActorLocation _playeroperatorref) _playeroperatorref (Variables|Default|GetAcceptanceRadius) false
        (:OnSuccess
          _)
        (:OnFail
          _))
      (Default|ChaseCompleted CallingTask))))

(event Custom|Wander
  (params (CallingTask :type STT%20Wander%20Object%20Reference))
  (bind _controlledenemycharacter (Variables|Default|GetControlledEnemyCharacter))
  (bind (_randomlocation _returnvalue) (Class|NavigationSystemV1|GetRandomLocationinNavigableRadius (Transformation|GetActorLocation _controlledenemycharacter) 1e+03 0 0))
  (if _returnvalue
    (AI|AIMoveTo _controlledenemycharacter _randomlocation 0 (Variables|Default|GetAcceptanceRadius) false
      (:OnSuccess
        _)
      (:OnFail
        _)))
  (Default|WanderCompleted CallingTask))

(event EventBeginPlay
  (bind _asfpcoperator (Utilities|Casting|CastToFPCOperator (Pawn|GetControlledPawn (Game|GetPlayerController 0))))
  (Variables|Default|SetPlayerOperatorRef _asfpcoperator))

(event EventTick
  (params (DeltaSeconds :type Float%20%28single-precision%29))
  (Variables|Default|SetWithinAttackDistance (< (Math|Vector|Distance(Vector) (Transformation|GetActorLocation (Variables|Default|GetPlayerOperatorRef)) (Transformation|GetActorLocation (Variables|Default|GetControlledEnemyCharacter))) 1.1e+02)))

(event EventPossess
  (params (PossessedPawn :type Pawn%20Object%20Reference))
  (bind _asbp_enemy_character_base (Utilities|Casting|CastToBP_EnemyCharacter_Base (Pawn|GetControlledPawn)))
  (Variables|Default|SetControlledEnemyCharacter _asbp_enemy_character_base))

(fn ConstructionScript)
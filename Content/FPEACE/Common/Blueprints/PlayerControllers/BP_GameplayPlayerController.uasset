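; BP_GameplayPlayerController is the gameplay player controller, handling input mode and the switch to the game over screen.
; BeginPlay sets game-only input and flushes pending input.
; OnGameOver removes all HUD, adds WBP_GameOverScreen to the viewport and opens it with the score and survival time from the controlled pawn's FPCPlayerState.
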(event Custom|OnGameOver
  (Class|FPCGameplayPlayerController|RemoveAllHUD)
  (bind _returnvalue (UserInterface|CreateWidget "/Game/FPEACE/Art/UI/Widgets/GameScreens/WBP_GameOverScreen.WBP_GameOverScreen_C"))
  (UserInterface|Viewport|AddtoViewport _returnvalue 0)
  (bind _asfpcplayer_state (Utilities|Casting|CastToFPCPlayerState (Variables|/Script/Engine.Pawn|GetPlayerState (Pawn|GetControlledPawn))))
  (Default|OpenGameOverScreen _returnvalue (Variables|/Script/Engine.PlayerState|GetScore _asfpcplayer_state) (Variables|/Script/FPEACE.FPCPlayerState|GetSurvivalTimeSeconds _asfpcplayer_state)))

(event EventBeginPlay
  (Input|SetInputModeGameOnly self true))

(fn ConstructionScript)